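; BP_Enemy_Base is a base enemy character that provides sword combat, patrol route access and movement speed control.
; WieldSword spawns a BP_EnemySword, snaps it to the right-hand mesh socket and flags the enemy as armed.
; Attack plays a sword-and-shield slash montage and calls OnAttackEnd on either completion or interruption.
; SetMovementSpeed maps a movement state to max walk speed, while GetPatrolRoute exposes the assigned route.
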(event `self.ReceiveBeginPlay`)

(event `Attack`
  (`|PlayMontage` (`self.Mesh`) "/Game/Characters/Mannequins/Animations/Manny/AM_Sword_And_Shield_Slash_Anim1_Montage.AM_Sword_And_Shield_Slash_Anim1_Montage"
    (:`OnCompleted`
      _)
    (:`OnInterrupted`
      _))
  (`self.OnAttackEnd`))

(event `WieldSword`
  (bind _returnvalue (`|SpawnActorFromClass` "/Game/Weapon/BP_EnemySword.BP_EnemySword_C" (`self.GetTransform`) "AlwaysSpawn" "MultiplyWithRoot" null null))
  (`self.K2_AttachToComponent` _returnvalue (`self.Mesh`) "hand_r_sword_socket" "SnapToTarget" "SnapToTarget" "SnapToTarget" true)
  (set `self.IsWieldingSword` true))

(fn `GetPatrolRoute`
  (returns (PatrolRoute :type "/Game/Enemies/BP_PatrolRoute Object Reference"))
  (return (`self.PatrolRoute`)))

(fn `SetMovementSpeed`
  (params (State :type "/Game/Enemies/Enums/E_MovementState Enum" :default "NewEnumerator0"))
  (returns (Speed :type "Float (double-precision)"))
  (bind _output_get (set `CharacterMovementComponent.MaxWalkSpeed` (select `/Game/Enemies/Enums/E_MovementState` State :`NewEnumerator1` 100.0 :`NewEnumerator2` 300.0 :`NewEnumerator3` 500.0) (`self.CharacterMovement`)))
  (return _output_get))

(fn `UserConstructionScript`)
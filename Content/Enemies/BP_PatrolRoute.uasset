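; BP_PatrolRoute is an enemy patrol path that supplies spline points as back-and-forth waypoints.
; IncrementPatrolRoute steps PatrolIndex by Direction along the PatrolRoute spline, flipping Direction at the last point and again at the first for a ping-pong loop.
; GetSplinePointAsWorld returns the world location of the spline point at the current index.
; The route keeps the index and direction state itself and contains no movement logic.
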(event `IncrementPatrolRoute`
  ; 적이 스플라인을 따라 이동해서 끝까지 갔는지 확인
  (bind _output_get (set `self.PatrolIndex` (+ (`self.PatrolIndex`) (`self.Direction`))))
  (if (== _output_get (- (`SplineComponent.GetNumberOfSplinePoints` (`self.PatrolRoute`)) 1))
    ; 참이면 되돌아 간다
    (set `self.Direction` -1)
    (else
      ; 되돌아 가서 다시 원점으로 오면 다시 반대로 이동
      (if (== (`self.PatrolIndex`) 0)
        (set `self.Direction` 1)))))

(fn `GetSplinePointAsWorld`
  (returns (Location :type "Vector Structure"))
  (return (`SplineComponent.GetLocationAtSplinePoint` (`self.PatrolRoute`) (`self.PatrolIndex`) "World")))

(fn `UserConstructionScript`)
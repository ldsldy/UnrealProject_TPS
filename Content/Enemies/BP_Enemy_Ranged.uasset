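; Ranged enemy character that wields a rifle and shoots at the attack target held by its AI controller.
; On BeginPlay it spawns the rifle and attaches it to a hand socket.
; DefaultAttack plays a fire montage whose notify calls the BPCAttacks component to fire a damaging bullet from weapon to target, signalling attack end on completion or interruption.
; It also supplies movement speeds per state, fixed ideal ranges and an IsDead that always returns false.
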(event `self.ReceiveBeginPlay`
  (`parent.ReceiveBeginPlay`)
  (`self.EquipWeapon`))

(event `/Game/Enemies/Interfaces/BPI_EnemyAI.EquipWeapon`
  (bind _returnvalue (`|SpawnActorFromClass` "/Game/Weapon/BP_Weapon_Rifle.BP_Weapon_Rifle_C" (`KismetMathLibrary.MakeTransform` (0.0 0.0 0.0)) "Undefined" "MultiplyWithRoot" null null))
  (bind _output_get (set `self.WeaponActor` _returnvalue))
  (`self.K2_AttachToComponent` _output_get (`self.Mesh`) "hand_r_rifle_socket" "SnapToTarget" "SnapToTarget" "SnapToTarget" true)
  (set `self.IsWieldingWeapon` true)
  (`self.OnWeaponEquipped`))

(event `/Game/Enemies/Interfaces/BPI_EnemyAI.DefaultAttack`
  (set `self.Attacking` true)
  (bind _notifyname (`|PlayMontage` (`self.Mesh`) "/Game/Animations/AM_Rifle_Fire.AM_Rifle_Fire")
    (:`OnCompleted`
      (`self.OnAttackEnd` :!label _label)
      (set `self.Attacking` false))
    (:`OnInterrupted`
      (goto _label))
    (:`OnNotifyBegin`
      (switch `name` _notifyname
        (:`Fire`
          (bind _asaic_enemy_base (cast `/Game/Enemies/AI/AIC_Enemy_Base` (`AIBlueprintHelperLibrary.GetAIController` self)))
          (bind _attacktarget (`/Game/Enemies/AI/AIC_Enemy_Base.AttackTarget` _asaic_enemy_base)
            (:`then`
              (`/Game/Attacks/BPC_Attacks.FireBullet` (`self.BPC_Attacks`) (`self.K2_GetActorLocation` (`self.WeaponActor`)) (`self.K2_GetActorLocation` _attacktarget) (make `/Game/DamageSystem/Structure/S_DamageInfo` 15.0 "NewEnumerator2")))
            (:`else`)))))))

(fn `GetIdealRange`
  (returns (AttackRadius :type "Float (double-precision)") (DefenseRadius :type "Float (double-precision)"))
  (return 600.0 600.0))

(fn `IsDead`
  (returns (IsDead :type Boolean))
  (return false))

(fn `SetMovementSpeed`
  (params (State :type "/Game/Enums/E_MovementState Enum" :default "NewEnumerator0"))
  (returns (Speed :type "Float (double-precision)"))
  (set `CharacterMovementComponent.MaxWalkSpeed` (select `/Game/Enums/E_MovementState` State :`NewEnumerator1` 200.0 :`NewEnumerator2` 300.0 :`NewEnumerator3` 500.0) (`self.CharacterMovement`))
  (return 0.0))

(fn `UserConstructionScript`
  (`parent.UserConstructionScript`))